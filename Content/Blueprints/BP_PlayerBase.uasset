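; Player base for a 2D side-scrolling platformer with flipbook idle, walk and jump animation, locked to its starting Y position.
; Tick picks the flipbook, faces the controller along X velocity, and runs a capsule trace while falling to detect wall slides.
; Wall slides lower gravity and refund one jump, feeding jump input that chooses ground, air or wall jumps via launches.
; Entering Walking at reduced speed restores normal speed after a delay.
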(event `self.ReceiveBeginPlay`
  (bind (_returnvalue_x _returnvalue_y) (`KismetMathLibrary.BreakVector` (`self.K2_GetActorLocation`)))
  (`|ExecutionSequence`
    (:`then_0`
      ;[1 1 1] Jump Gravity
      (set `self.DefaultGravity` (`CharacterMovementComponent.GravityScale` (`self.CharacterMovement`))))
    (:`then_1`
      ;[1 1 1] Constrain Y Axis
      (set `self.LevelYPOS` _returnvalue_y))))

(event `Reset PlayerYPOS`
  (bind (_returnvalue_x _returnvalue_y _returnvalue_z) (`KismetMathLibrary.BreakVector` (`self.K2_GetActorLocation`)))
  (bind (_returnvalue_x_2 _returnvalue_y_2) (`KismetMathLibrary.BreakVector` (`self.K2_GetActorLocation`)))
  ;[1 1 1] Constrain Y Axis
  (if (!= (`self.LevelYPOS`) _returnvalue_y_2)
    (`self.K2_SetActorLocation` (`KismetMathLibrary.MakeVector` _returnvalue_x (`self.LevelYPOS`) _returnvalue_z))))

(event `self.ReceiveTick`
  (params (DeltaSeconds :type "Float (single-precision)"))
  (bind (_returnvalue_x _returnvalue_y) (`KismetMathLibrary.BreakVector` (`self.GetVelocity`)))
  (bind _returnvalue_x_2 (`KismetMathLibrary.BreakVector` (`self.GetVelocity`)))
  (bind (_returnvalue_x_3 _returnvalue_y_2 _returnvalue_z) (`KismetMathLibrary.BreakVector` (`self.GetVelocity`)))
  (bind _returnvalue (`self.K2_GetActorLocation`))
  (bind (_returnvalue_x_4 _returnvalue_y_3 _returnvalue_z_2) (`KismetMathLibrary.BreakVector` (`self.GetVelocity`)))
  ;[1 1 1] Handle
  (`|ExecutionSequence`
    (:`then_0`
      ;[1 1 1] Sprite Animation
      (if (`NavMovementComponent.IsFalling` (`self.CharacterMovement`))
        (`PaperFlipbookComponent.SetFlipbook` (`self.Sprite`) (`self.FB_Jump`))
        (elif (!= (`KismetMathLibrary.VSize` (`self.GetVelocity`)) 0.0)
          (`PaperFlipbookComponent.SetFlipbook` (`self.Sprite`) (`self.FB_Walk`))
          (else
            (`PaperFlipbookComponent.SetFlipbook` (`self.Sprite`) (`self.FB_Idle`))))))
    (:`then_1`
      ;[1 1 1] Sprite Rotation
      (`/Engine/EditorBlueprintResources/StandardMacros.CompareFloat` _returnvalue_x_2
        (:`>`
          (`Controller.SetControlRotation` (`GameplayStatics.GetPlayerController` 0) (`KismetMathLibrary.MakeRotator` 0.0 0.0 0.0)))
        (:`<`
          (`Controller.SetControlRotation` (`GameplayStatics.GetPlayerController` 0) (`KismetMathLibrary.MakeRotator` 0.0 0.0 180.0)))))
    (:`then_2`
      ;[1 1 1] Constrain Y Axis
      (`self.Reset PlayerYPOS`))
    (:`then_3`
      ;[1 1 1] WallSlide
      (if (`NavMovementComponent.IsFalling` (`self.CharacterMovement`))
        (bind _outhit (`KismetSystemLibrary.CapsuleTraceSingle` :`Start` _returnvalue :`End` _returnvalue :`Radius` 56.0 :`HalfHeight` 88.0 :`TraceChannel` "TraceTypeQuery1" :`DrawDebugType` "ForOneFrame"))
        (set `self.bInWallslide` (`GameplayStatics.BreakHitResult` _outhit))
        (if (`GameplayStatics.BreakHitResult` _outhit)
          (set `self.JumpCount` (- (`self.JumpMaxCount`) 1))
          (if (<= _returnvalue_z_2 0.0)
            (`|ExecutionSequence`
              (:`then_0`
                (`/Engine/EditorBlueprintResources/StandardMacros.DoOnce` false :!label _label
                  (:`Completed`
                    (`/Engine/EditorBlueprintResources/StandardMacros.DoOnce` false
                      (:`Completed`
                        (set `MovementComponent.Velocity` (`KismetMathLibrary.MakeVector` _returnvalue_x _returnvalue_y) (`self.CharacterMovement`)))))))
              (:`then_1`
                (set `CharacterMovementComponent.GravityScale` 0.1 (`self.CharacterMovement`))
                (set `MovementComponent.Velocity` (`KismetMathLibrary.VInterpTo` (`self.GetVelocity`) (`KismetMathLibrary.MakeVector` 0.0 0.0 _returnvalue_z) (`GameplayStatics.GetWorldDeltaSeconds`) (`self.WallSlideDecelerationSpeed`)) (`self.CharacterMovement`))
                (bind (_returnvalue_roll _returnvalue_pitch _returnvalue_yaw) (`KismetMathLibrary.BreakRotator` (`KismetMathLibrary.Conv_VectorToRotator` (`.Normal` (`GameplayStatics.BreakHitResult` _outhit)))))
                (`self.K2_SetActorRotation` (`KismetMathLibrary.MakeRotator` 0.0 0.0 (+ _returnvalue_yaw 0.0))))))
          (else
            (set `CharacterMovementComponent.GravityScale` (`self.DefaultGravity`) (`self.CharacterMovement`))
            (`self.WallSlideVelocityReset`)))))))

(event `WallSlideVelocityReset`
  ;[1 1 1] WallSlide
  (goto _label :!via `Reset`))

(event `InputAxis|MoveRight`
  (params (AxisValue :type "Float (single-precision)"))
  ;[1 1 1] Base Movement
  (if (> AxisValue 0.0)
    (set `self.IsMovingRight?` true)
    (elif (< AxisValue 0.0)
      (set `self.IsMovingRight?` false)))
  (`self.AddMovementInput` (1.0 0.0 0.0) AxisValue))

(event `Handle Rotation`
  (bind _velocity_x (`KismetMathLibrary.BreakVector` (`MovementComponent.Velocity` (`self.CharacterMovement`))))
  ;[1 1 1] Character Rotation
  (`/Engine/EditorBlueprintResources/StandardMacros.CompareFloat` _velocity_x
    (:`>`
      (`Controller.SetControlRotation` (`self.GetController`) (`KismetMathLibrary.MakeRotator` 0.0) :!label _label_2))
    (:`==`
      (if (`self.IsMovingRight?`)
        (goto _label_2)
        (else
          (`Controller.SetControlRotation` (`self.GetController`) (`KismetMathLibrary.MakeRotator` 0.0 0.0 180.0) :!label _label_3))))
    (:`<`
      (goto _label_3))))

(event `InputAction|Jump`
  (params (Key :type "Key Structure"))
  ;[1 1 1] Jump & WallJump
  (:`Pressed`
    (if (< (`self.JumpCount`) (`self.JumpMaxCount`))
      (if (`NavMovementComponent.IsFalling` (`self.CharacterMovement`))
        (if (`self.bInWallslide`)
          ;;[1 1 1] Wall Jump
          (`self.LaunchCharacter` (+ (* (`self.GetActorForwardVector`) (`self.WallJumpForce`)) (`KismetMathLibrary.MakeVector` 0.0 0.0 (`self.AirJumpVelocity`))) true true)
          (else
            ;;[1 1 1] Air Jump
            (`self.LaunchCharacter` (+ (`self.GetVelocity`) (`KismetMathLibrary.MakeVector` 0.0 0.0 (`self.AirJumpVelocity`))) true true)
            (`/Engine/EditorBlueprintResources/StandardMacros.IncrementInt` (`self.JumpCount`))))
        (else
          ;;[1 1 1] Ground Jump
          (`self.Jump`)
          (`/Engine/EditorBlueprintResources/StandardMacros.IncrementInt` (`self.JumpCount`))))))
  (:`Released`
    (`self.StopJumping`)))

(event `self.OnLanded`
  (params (Hit :type "HitResult Structure (by ref)"))
  ;[1 1 1] Jump & WallJump
  (set `self.JumpCount` 0))

(event `self.K2_OnMovementModeChanged`
  (params (PrevMovementMode :type "EMovementMode Enum" :default "MOVE_None") (NewMovementMode :type "EMovementMode Enum" :default "MOVE_None") (PrevCustomMode :type Byte) (NewCustomMode :type Byte))
  (if (`|EnumEquality` NewMovementMode "MOVE_Walking")
    (if (== (`CharacterMovementComponent.MaxWalkSpeed` (`self.CharacterMovement`)) 200.0)
      (`/Engine/EditorBlueprintResources/StandardMacros.DoOnce` false :!label _label_4
        (:`Completed`
          (`KismetSystemLibrary.Delay` 5.0)
          (set `CharacterMovementComponent.MaxWalkSpeed` 600.0 (`self.CharacterMovement`))
          (goto _label_4 :!via `Reset`))))))

(fn `UserConstructionScript`)