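; A grow pickup that swaps the player's character for a BP_PlayerBase_03 when its box is overlapped.
; On overlap it destroys itself, records the location and rotation of player character 0, and destroys that character.
; It then spawns BP_PlayerBase_03 at the saved transform and calls PossessCharacter on it.
; The overlapping actor is not checked, so any overlap triggers the swap.
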(event `self.Box.OnComponentBeginOverlap`
  (params (OverlappedComponent :type "PrimitiveComponent Object Reference") (OtherActor :type "Actor Object Reference") (OtherComp :type "PrimitiveComponent Object Reference") (OtherBodyIndex :type Integer) (bFromSweep :type Boolean) (SweepResult :type "HitResult Structure (by ref)"))
  (bind _returnvalue (`GameplayStatics.GetPlayerCharacter` 0))
  (`self.K2_DestroyActor`)
  (set `self.Spawn Transform Location` (`self.K2_GetActorLocation` _returnvalue))
  (set `self.Set Spawn Rotation` (`self.K2_GetActorRotation` _returnvalue))
  (`self.K2_DestroyActor` _returnvalue)
  (bind _returnvalue_2 (`|SpawnActorFromClass` "/Game/Blueprints/BP_PlayerBase_03.BP_PlayerBase_03_C" (`KismetMathLibrary.MakeTransform` (`self.Spawn Transform Location`) (`self.Set Spawn Rotation`)) "Undefined" "OverrideRootScale" null null))
  (`/Game/Blueprints/BP_PlayerBase_03.Possess Character` _returnvalue_2))

(fn `UserConstructionScript`)